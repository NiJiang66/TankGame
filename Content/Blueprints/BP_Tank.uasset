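; Player-controlled tank Blueprint that wires input to its aiming and movement components.
; On BeginPlay it hands the barrel and turret to TankAiming, the two tracks to TankMovement, and itself to the HP bar widget.
; Move and Fire inputs are forwarded to those components.
; Look input yaws a scene component and pitches the spring arm within a clamped range for camera orbit.
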(event EventBeginPlay
  (Class|TankAimingComponent|Initialize (Variables|Default|GetTankAiming) (Variables|Default|GetTankBarrel) (Variables|Default|GetTankTurret))
  (Class|TankMovementComponent|Initialize (Variables|Default|GetTankMovement) (Variables|Default|GetLeftTrack) (Variables|Default|GetRightTrack))
  (bind _ashp_bar_bp (Utilities|Casting|CastToHpBar_BP (UserInterface|GetUserWidgetObject (Variables|Default|GetHPBarWidget))))
  (Variables|/Game/Blueprints/UI/HpBar_BP.HpBar_BP_C|SetTank _ashp_bar_bp self))

(event Input|ActionEvents|InputActionFire
  (params (Key :type Key%20Structure))
  (:Pressed
    (Class|TankAimingComponent|Fire (Variables|Default|GetTankAiming))))

(event Input|AxisEvents|InputAxisLookH
  (params (AxisValue :type Float%20%28single-precision%29))
  (Transformation|AddRelativeRotation (Variables|Default|GetScene) (Math|Rotator|MakeRotator 0.0 0.0 AxisValue) false false))

(event Input|AxisEvents|InputAxisLookV
  (params (AxisValue :type Float%20%28single-precision%29))
  (bind _springarm (Variables|Default|GetSpringArm))
  (bind _relativerotation (Variables|/Script/Engine.SceneComponent|GetRelativeRotation _springarm))
  (Transformation|SetRelativeRotation (Variables|Default|GetSpringArm) (Math|Rotator|MakeRotator (.roll _relativerotation) (Math|Float|Clamp(Float) (+ AxisValue (.pitch _relativerotation)) -4e+01 5.0) (.yaw _relativerotation)) false false))

(event Input|AxisEvents|InputAxisMoveForward
  (params (AxisValue :type Float%20%28single-precision%29))
  (Class|TankMovementComponent|MoveForward (Variables|Default|GetTankMovement) AxisValue))

(event Input|AxisEvents|InputAxisMoveRight
  (params (AxisValue :type Float%20%28single-precision%29))
  (Class|TankMovementComponent|MoveRight (Variables|Default|GetTankMovement) AxisValue))

(fn ConstructionScript)